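; BP_GodAIController is a controller that drives an SLGod pawn with simple per-tick movement and turning.
; BeginPlay caches the controlled pawn as an SLGod.
; Each tick, CanMove feeds half-scale movement input along the X and Y of the pawn camera's forward vector.
; CanTurn sets the actor's rotation to its control rotation plus a delta-time-scaled yaw offset.
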(event EventBeginPlay
  (bind _asslgod (Utilities|Casting|CastToSLGod (Pawn|GetControlledPawn))))

(event EventTick
  (params (DeltaSeconds :type Float%20%28single-precision%29))
  (if (Variables|/Script/SMITElabs.SLGod|GetbCanMove (stale EventBeginPlay _asslgod))
    (Pawn|Input|AddMovementInput (stale EventBeginPlay _asslgod) (Math|Vector|MakeVector (.x (Math|Vector|GetForwardVector (Variables|/Script/SMITElabs.SLGod|GetCameraComponent (stale EventBeginPlay _asslgod)))) (.y (Math|Vector|GetForwardVector (Variables|/Script/SMITElabs.SLGod|GetCameraComponent (stale EventBeginPlay _asslgod)))) 0.0) 0.5 false))
  (if (Variables|/Script/SMITElabs.SLGod|GetbCanTurn (stale EventBeginPlay _asslgod))
    (Transformation|SetActorRotation (stale EventBeginPlay _asslgod) (Math|Rotator|MakeRotator (.roll (Pawn|GetControlRotation (stale EventBeginPlay _asslgod) :!class /Script/Engine.Pawn)) (.pitch (Pawn|GetControlRotation (stale EventBeginPlay _asslgod) :!class /Script/Engine.Pawn)) (+ (.yaw (Pawn|GetControlRotation (stale EventBeginPlay _asslgod) :!class /Script/Engine.Pawn)) (* (Utilities|Time|GetWorldDeltaSeconds) 9e+01))))))

(fn ConstructionScript)